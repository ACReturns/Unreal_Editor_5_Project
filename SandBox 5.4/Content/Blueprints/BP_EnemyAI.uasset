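; Enemy AI character that chases the player on sight, plays a montage on reaching them and takes damage.
; PawnSensing triggers AIMoveTo toward the player; CanAttack halts movement during the montage.
; AnyDamage lowers Health, shown on a widget health bar also refreshed every Tick, and destroys the actor on a hit arriving below 1 health.
; Waypoint patrol logic exists but is never started; overlap damage test is disabled.
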(event `self.ReceiveBeginPlay`
  (`self.UpdateHealthBar`))

(event `self.ReceiveAnyDamage`
  (params (Damage :type "Float (single-precision)") (DamageType :type "DamageType Object Reference") (InstigatedBy :type "Controller Object Reference") (DamageCauser :type "Actor Object Reference"))
  (bind _health (`self.Health`))
  ;[1 1 1] Damage Enemy
  (set `self.DamageTaken` Damage)
  (if (>= _health 1.0)
    (set `self.Health` (- _health (`self.DamageTaken`)))
    (`self.UpdateHealthBar`)
    (`KismetSystemLibrary.PrintString` (`KismetStringLibrary.Concat_StrStr` "Damage Taken: " (`KismetStringLibrary.Conv_DoubleToString` (`self.DamageTaken`))))
    (else
      (`self.K2_DestroyActor`))))

(event `self.ReceiveTick`
  (params (DeltaSeconds :type "Float (single-precision)"))
  ;[1 1 1] Tracking
  (`self.UpdateHealthBar`)
  (if (not (`self.CanAttack`))
    (`MovementComponent.StopMovementImmediately` (`self.CharacterMovement`))))

(event `self.PawnSensing.OnSeePawn`
  (params (Pawn :type "Pawn Object Reference"))
  ;[1 1 1] Track Player
  (set `self.isSeeingPlayer` true)
  (`self.Follow Player`))

(event `Follow Player`
  ;[1 1 1] Track Player
  (set `self.CanAttack` true)
  (if (`self.isSeeingPlayer`)
    (`|AIMoveTo` self (0.0 0.0 0.0) (`GameplayStatics.GetPlayerCharacter` 0) (`self.Player Distance`)
      (:`OnSuccess`
        (if (`self.CanAttack`)
          (set `self.CanAttack` false)
          (bind _returnvalue (`self.PlayAnimMontage` null))
          (`KismetSystemLibrary.Delay` _returnvalue)
          (set `self.CanAttack` true))))
    (else
      (set `self.isSeeingPlayer` false))))

(event `Patrol`
  (bind _locations (`self.Locations`))
  ;[1 1 1] Patrol
  (set `CharacterMovementComponent.MaxWalkSpeed` 150.0 (`self.CharacterMovement`))
  (`|AIMoveTo` self (`|GetArrayItem` (`self.PatrolLocation`) (`self.Locations`)) null
    (:`OnSuccess`
      (`KismetSystemLibrary.Delay` (`KismetMathLibrary.RandomFloatInRange` 1.0 3.0))
      (`self.Patrol`)
      (`/Engine/EditorBlueprintResources/StandardMacros.IncrementInt` _locations
        (:`  `
          (if (== _locations 2)
            (set `self.Locations` 0)))))))

(fn `UpdateHealthBar`
  (bind _asw_aihealth_bar (cast `/Game/HUD/W_AIHealthBar` (`WidgetComponent.GetUserWidgetObject` (`self.HealthBar`))))
  (set `/Game/HUD/W_AIHealthBar.Health` (`self.Health`) _asw_aihealth_bar)
  (return))

(fn `UserConstructionScript`)