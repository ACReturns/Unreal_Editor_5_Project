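; BP_CameraManager is a camera follow actor that smoothly tracks the FollowPlayer actor.
; Each tick, UpdateCameraPosition interpolates its location toward the player's position plus a look-ahead offset scaled by CameraOffset along the player's forward vector.
; The offset ignores the Y axis, and LockHeight keeps the actor's current Z as the base height in place of the player's.
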(event `self.ReceiveTick`
  (params (DeltaSeconds :type "Float (single-precision)"))
  (`self.Update Camera Position`))

(fn `Update Camera Position`
  (bind (_returnvalue_x _returnvalue_y _returnvalue_z) (`KismetMathLibrary.BreakVector` (`self.K2_GetActorLocation`)))
  (bind (_returnvalue_x_2 _returnvalue_y_2 _returnvalue_z_2) (`KismetMathLibrary.BreakVector` (`self.K2_GetActorLocation` (`self.Follow Player`))))
  (bind (_returnvalue_x_3 _returnvalue_y_3 _returnvalue_z_3) (`KismetMathLibrary.BreakVector` (* (`self.GetActorForwardVector` (`self.Follow Player`)) (`self.Camera Offset`))))
  (`self.K2_SetActorLocation` (`KismetMathLibrary.VInterpTo` (`self.K2_GetActorLocation`) (+ (`KismetMathLibrary.MakeVector` _returnvalue_x_2 _returnvalue_y_2 (select `bool` (`self.Lock Height`) :`false` _returnvalue_z_2 :`true` _returnvalue_z)) (`KismetMathLibrary.MakeVector` _returnvalue_x_3 0.0 _returnvalue_z_3)) (`GameplayStatics.GetWorldDeltaSeconds`) (`self.Interp Speed`))))

(fn `UserConstructionScript`)